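; BP_BlueBallSocket is a puzzle socket that counts toward opening a linked Door when a blue object enters it.
; Its Box overlap event checks the other actor for the "Blue" tag, increments the Door's CompletedToggles and calls CheckCompletedToggles on it.
; Nothing guards against repeat overlaps or decrements the count on exit, and a leftover counter-and-print branch is never run.
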(event OnComponentBeginOverlap(Box)
  (params (OverlappedComponent :type Primitive%20Component%20Object%20Reference) (OtherActor :type Actor%20Object%20Reference) (OtherComp :type Primitive%20Component%20Object%20Reference) (OtherBodyIndex :type Integer) (bFromSweep :type Boolean) (SweepResult :type Hit%20Result%20Structure%20%28by%20ref%29))
  (bind _door (Variables|Default|GetDoor))
  (if (Actor|ActorHasTag OtherActor "Blue")
    (Utilities|IsValid OtherActor
      (:Is%20Valid
        (Math|Integer|IncrementInt (Variables|/Game/StudentWork/BP_LockedDoor.BP_LockedDoor_C|GetCompletedToggles _door)
          (:%20%20
            (Default|CheckCompletedToggles _door)))))))

(event EventBeginPlay)

(event Collision|EventActorBeginOverlap
  (params (OtherActor :type Actor%20Object%20Reference)))

(event EventTick
  (params (DeltaSeconds :type Float%20%28single-precision%29)))

(fn ConstructionScript)