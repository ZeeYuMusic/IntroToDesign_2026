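; BP_LockedDoor is a door that slides open once enough toggles are completed and slides closed otherwise.
; CheckCompletedToggles prints CompletedToggles, compares it with RequiredToggles, then plays or reverses a Timeline that lerps the mesh between its BeginPlay location and that location plus DoorOffset.
; The count is not incremented here, and ResetCompletedTogglesCount zeroes it and re-runs the check.
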(event Custom|CheckCompletedToggles
  (bind _completedtoggles (Variables|Default|GetCompletedToggles))
  (Development|PrintString (Utilities|String|ToString(Integer) _completedtoggles))
  (if (>= _completedtoggles (Variables|Default|GetRequiredToggles))
    (CallFunction|OpenDoor)
    (else
      (CallFunction|ClosedDoor))))

(event Custom|OpenDoor
  (bind _start_location (Variables|Default|GetStart%20Location))
  (bind _alpha (Timeline|Timeline Play)
    (:Update
      (Transformation|SetWorldLocation (Variables|Default|GetStatic%20Mesh) (Math|Vector|Lerp(Vector) _start_location (+ _start_location (Variables|Default|GetDoor%20Offset)) _alpha) false false))))

(event Custom|ClosedDoor
  (bind _start_location (Variables|Default|GetStart%20Location))
  (bind _alpha (Timeline|Timeline Reverse)
    (:Update
      (Transformation|SetWorldLocation (Variables|Default|GetStatic%20Mesh) (Math|Vector|Lerp(Vector) _start_location (+ _start_location (Variables|Default|GetDoor%20Offset)) _alpha) false false))))

(event Custom|ResetCompletedTogglesCount
  (Variables|Default|SetCompletedToggles 0)
  (CallFunction|CheckCompletedToggles))

(event EventBeginPlay
  (Variables|Default|SetStart%20Location (Transformation|GetWorldLocation (Variables|Default|GetStatic%20Mesh))))

(event EventTick
  (params (DeltaSeconds :type Float%20%28single-precision%29)))

(fn ConstructionScript)