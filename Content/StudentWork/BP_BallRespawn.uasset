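; Damage-triggered reset actor that respawns two puzzle balls and resets the linked Door's completed-toggle count.
; BeginPlay caches the starting locations of BSphere and YSphere.
; AnyDamage passes through a DoOnce, then destroys both balls, spawns BP_BlueSphere and BP_RedSphere at those locations, and stores the new references.
; The sequence ends by calling ResetBallResetDoOnce, re-arming the gate for the next hit.
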(event Custom|ResetBallResetDoOnce
  (Utilities|FlowControl|DoOnce false) ; enters at Reset
)

(event EventBeginPlay
  (Variables|Default|SetBSphereSpawn (Transformation|GetWorldLocation (Variables|/Script/Engine.Actor|GetRootComponent (Variables|Default|GetBSphere))))
  (Variables|Default|SetYSphereSpawn (Transformation|GetWorldLocation (Variables|/Script/Engine.Actor|GetRootComponent (Variables|Default|GetYSphere)))))

(event Game|Damage|EventAnyDamage
  (params (Damage :type Float%20%28single-precision%29) (DamageType :type Damage%20Type%20Object%20Reference) (InstigatedBy :type Controller%20Object%20Reference) (DamageCauser :type Actor%20Object%20Reference))
  (Utilities|FlowControl|DoOnce false
    (:Completed
      (Actor|DestroyActor (Variables|Default|GetBSphere))
      (bind _returnvalue (Game|SpawnActorfromClass "/Game/StudentWork/BP_BlueSphere.BP_BlueSphere_C" (Math|Transform|MakeTransform (Variables|Default|GetBSphereSpawn) "0, 0, 0" "1.000000,1.000000,1.000000") "Undefined" "MultiplyWithRoot" 0 0))
      (Variables|Default|SetBSphere _returnvalue)
      (Actor|DestroyActor (Variables|Default|GetYSphere))
      (bind _returnvalue_2 (Game|SpawnActorfromClass "/Game/StudentWork/BP_RedSphere.BP_RedSphere_C" (Math|Transform|MakeTransform (Variables|Default|GetYSphereSpawn) "0, 0, 0" "1.000000,1.000000,1.000000") "Undefined" "MultiplyWithRoot" 0 0))
      (Variables|Default|SetYSphere _returnvalue_2)
      (Default|ResetCompletedTogglesCount (Variables|Default|GetDoor))
      (CallFunction|ResetBallResetDoOnce))))

(fn ConstructionScript)