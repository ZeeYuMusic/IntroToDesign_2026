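; BP_Door is a sliding door that opens when the player character steps into its trigger box and closes when they leave.
; BeginPlay caches the static mesh's world location as the closed position.
; Box overlap events play or reverse a Timeline, whose Alpha lerps the mesh between that start location and the start plus DoorOffset.
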(event OnComponentBeginOverlap(Box)
  (params (OverlappedComponent :type Primitive%20Component%20Object%20Reference) (OtherActor :type Actor%20Object%20Reference) (OtherComp :type Primitive%20Component%20Object%20Reference) (OtherBodyIndex :type Integer) (bFromSweep :type Boolean) (SweepResult :type Hit%20Result%20Structure%20%28by%20ref%29))
  (bind _start_location (Variables|Default|GetStart%20Location))
  (Utilities|Casting|CastToPlayerCharacter OtherActor)
  (bind _alpha (Timeline|Timeline Play)
    (:Update
      (Transformation|SetWorldLocation (Variables|Default|GetStatic%20Mesh) (Math|Vector|Lerp(Vector) _start_location (+ _start_location (Variables|Default|GetDoor%20Offset)) _alpha) false false))))

(event OnComponentEndOverlap(Box)
  (params (OverlappedComponent :type Primitive%20Component%20Object%20Reference) (OtherActor :type Actor%20Object%20Reference) (OtherComp :type Primitive%20Component%20Object%20Reference) (OtherBodyIndex :type Integer))
  (bind _start_location (Variables|Default|GetStart%20Location))
  (Utilities|Casting|CastToPlayerCharacter OtherActor)
  (bind _alpha (Timeline|Timeline Reverse)
    (:Update
      (Transformation|SetWorldLocation (Variables|Default|GetStatic%20Mesh) (Math|Vector|Lerp(Vector) _start_location (+ _start_location (Variables|Default|GetDoor%20Offset)) _alpha) false false))))

(event EventBeginPlay
  (Variables|Default|SetStart%20Location (Transformation|GetWorldLocation (Variables|Default|GetStatic%20Mesh))))

(event EventTick
  (params (DeltaSeconds :type Float%20%28single-precision%29)))

(fn ConstructionScript)